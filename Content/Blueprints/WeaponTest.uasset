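; WeaponTest is a prototype hitscan weapon owned by the player, fired through its UseWeapon event.
; UseWeapon casts the owner to PlayerBP and runs a Visibility line trace from the player camera along its forward vector, out to Range.
; A hit actor implementing LB_IShootable receives ShotMessage, so targets define their own reaction.
; The trace draws persistent debug lines.
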(event Custom|UseWeapon
  (bind _asplayer_bp (Utilities|Casting|CastToPlayerBP (Components|GetOwner)))
  (bind _outhit (Collision|LineTraceByChannel (Transformation|GetWorldLocation (Variables|/Script/ZombieShooter.PlayerCharacter|GetPlayerCamera _asplayer_bp)) (+ (Transformation|GetWorldLocation (Variables|/Script/ZombieShooter.PlayerCharacter|GetPlayerCamera _asplayer_bp)) (* (Math|Vector|GetForwardVector (Variables|/Script/ZombieShooter.PlayerCharacter|GetPlayerCamera _asplayer_bp)) (Variables|Default|GetRange))) "TraceTypeQuery1" false 0 "Persistent"))
  (if (Utilities|DoesObjectImplementInterface (.hitactor _outhit) "/Script/ZombieShooter.LB_IShootable")
    (Class|LBIShootable|Shot(Message) (.hitactor _outhit))))

(event EventBeginPlay)

(event EventTick
  (params (DeltaSeconds :type Float%20%28single-precision%29)))