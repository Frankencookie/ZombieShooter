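; Player Blueprint that sets up the HUD and first weapon viewmodel, and handles interaction feedback.
; On BeginPlay it creates the HUD widget with the hand hidden, then applies the first equipped weapon's static model from the weapon component to the viewmodel mesh, printing that model's name.
; The CanInteract event shows the HUD hand.
; The construction script assigns the weapon component to a variable.
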(event EventBeginPlay
  (bind _weaponcomponent1 (Variables|Default|GetWeaponComponent1))
  (bind _equippedweapons (Variables|/Script/ZombieShooter.LB_WeaponComponent|GetEquippedWeapons _weaponcomponent1))
  (bind _output (Utilities|Array|Get(acopy) _equippedweapons))
  (bind _weapondata (Variables|/Script/ZombieShooter.WeaponBehaviour|GetWeaponData _output))
  (bind _staticweaponmodel (Variables|/Script/ZombieShooter.LB_WeaponData|GetStaticWeaponModel _weapondata))
  (Utilities|FlowControl|Sequence
    (:then_0
      (bind _returnvalue (UserInterface|CreateWidget "/Game/UI/HUD.HUD_C" (Game|GetPlayerController 0)))
      (UserInterface|Viewport|AddtoViewport _returnvalue 0)
      (Default|HandHide _returnvalue)
      (Variables|Default|SetHUD%20Ref _returnvalue))
    (:then_2
      (Development|PrintString (Utilities|GetDisplayName _staticweaponmodel))
      ;[1 1 1] Set up weapon mesh
      (Components|StaticMesh|SetStaticMesh (Variables|Default|GetWeaponViewmodel) _staticweaponmodel))))

(event EventCanInteract
  (Default|ShowHand (Variables|Default|GetHUD%20Ref)))

(fn ConstructionScript
  (Variables|Default|SetWeaponComponent (Variables|Default|GetWeaponComponent1)))