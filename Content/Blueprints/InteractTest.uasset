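; InteractTest is an interactable test actor whose Cube rotates open once when the player interacts with it.
; BeginPlay caches the cube's starting world rotation.
; Interacted sets Opened and plays a timeline that adds its Rotate track to the starting yaw.
; GetCanInteract returns true only while Opened is false, so the interaction cannot repeat.
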(event EventBeginPlay
  (Variables|Default|SetStartRot (Transformation|GetWorldRotation (Variables|Default|GetCube))))

(event Collision|EventActorBeginOverlap
  (params (OtherActor :type Actor%20Object%20Reference)))

(event EventTick
  (params (DeltaSeconds :type Float%20%28single-precision%29)))

(event EventInteracted
  (bind _startrot (Variables|Default|GetStartRot))
  (Variables|Default|SetOpened true)
  (bind _rotate (Timeline|Timeline_0 Play)
    (:Update
      (Transformation|SetWorldRotation (Variables|Default|GetCube) (Math|Rotator|MakeRotator (.roll _startrot) (.pitch _startrot) (+ (.yaw _startrot) _rotate)) false false))))

(fn ConstructionScript)

(fn GetCanInteract
  (return (not (Variables|Default|GetOpened))))